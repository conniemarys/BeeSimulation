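; BP_HexGrid is a grid actor that lays out a Width by Height field of hex tiles in its construction script.
; It spaces tiles by a radius taken from the TileMesh bounding box plus an Offset gap, with a FlipFlop staggering rows by one radius.
; The Instanced flag selects between instances of TileMesh on an InstancedStaticMesh and BP_CubeTile child actors.
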(fn `UserConstructionScript`
  (bind _offset (`self.Offset`))
  (bind _tilemesh (`self.TileMesh`))
  (`StaticMeshComponent.SetStaticMesh` (`self.InstancedStaticMesh`) _tilemesh)
  (set `self.Radius` (.x (`.Max` (break `Box` (`StaticMesh.GetBoundingBox` _tilemesh)))))
  ;[1 1 1] Height Loop
  (for _index (range 1 (+ (`self.Height`) 1))
    ;[1 1 1] Width Loop
    (for _index_2 (range 1 (+ (`self.Width`) 1))
      (if (`self.Instanced?`)
        (bind _returnvalue (+ (`self.RowOffset`) (* _index_2 (`self.Radius`) 2.0) (* _index_2 _offset)))
        (bind _returnvalue_2 (+ (* _offset _index) (* _index 1.5 (/ (* (`self.Radius`) 2.0) (`KismetMathLibrary.Sqrt` 3.0)))))
        ;[1 1 1] Instanced Mesh
        (`InstancedStaticMeshComponent.AddInstance` (`self.InstancedStaticMesh`) (`KismetMathLibrary.MakeTransform` (`KismetMathLibrary.MakeVector` _returnvalue _returnvalue_2)) false)
        (else
          ;[1 1 1] Child Actors
          (bind _returnvalue_3 (`AddComponent|NODE_AddChildActorComponent-0` :`RelativeTransform` (`KismetMathLibrary.MakeTransform` (`KismetMathLibrary.MakeVector` _returnvalue _returnvalue_2))))
          (`ChildActorComponent.SetChildActorClass` _returnvalue_3 "/Game/GridSystem/BP_CubeTile.BP_CubeTile_C"))))
    (`/Engine/EditorBlueprintResources/StandardMacros.FlipFlop`
      (:`A`
        (set `self.RowOffset` (* (`self.Radius`) -1.0)))
      (:`B`
        (set `self.RowOffset` 0.0)))))