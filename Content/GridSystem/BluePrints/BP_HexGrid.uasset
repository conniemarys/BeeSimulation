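; BP_HexGrid is an actor that builds a Width by Height hex tile grid with walls in its construction script.
; SpawnArrays fills a 2D struct array of cells, each with a random wall side.
; SpawnGrid staggers alternate rows by the tile mesh radius, placing tiles and walls as mesh instances or child actors per the Instanced flag.
; Wall offsets come from a data table; the child-actor path always uses NorthEast.
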(event `self.ReceiveBeginPlay`)

(event `self.ReceiveTick`
  (params (DeltaSeconds :type "Float (single-precision)")))

(event `InitialSpawn`)

(fn `CreateCellTransform`
  (params (XIndex :type Integer) (YIndex :type Integer))
  (returns (ReturnValue :type "Transform Structure"))
  (bind _xindex (`local.XIndex`))
  (bind _offset (`self.Offset`))
  (bind _yindex (`local.YIndex`))
  (return (`KismetMathLibrary.MakeTransform` (`KismetMathLibrary.MakeVector` (+ (`self.RowOffset`) (* _yindex (`self.Radius_0`) 2.0) (* _yindex _offset)) (+ (* _offset _xindex) (* _xindex 1.5 (/ (* (`self.Radius_0`) 2.0) (`KismetMathLibrary.Sqrt` 3.0))))))))

(fn `DestroyInstances`
  (if (!= (`KismetArrayLibrary.Array_Length` (`self.TileInstances`)) 0)
    (`InstancedStaticMeshComponent.RemoveInstances` (`self.HexTileInstance`) (`self.TileInstances`)))
  (if (!= (`KismetArrayLibrary.Array_Length` (`self.WallInstances`)) 0)
    (`InstancedStaticMeshComponent.RemoveInstances` (`self.WallInstance`) (`self.WallInstances`))
    (`KismetArrayLibrary.Array_Clear` (`self.TileInstances`))
    (`KismetArrayLibrary.Array_Clear` (`self.WallInstances`))))

(fn `GetRandomWallSides`
  (returns (WallSides :type "/Game/GridSystem/StructsAndDataTables/ENUM_WallSides Enum"))
  (switch `int` (`KismetMathLibrary.RandomIntegerInRange` 0 5)
    (:`0`
      (return "NewEnumerator0"))
    (:`1`
      (return "NewEnumerator1"))
    (:`2`
      (return "NewEnumerator2"))
    (:`3`
      (return "NewEnumerator3"))
    (:`4`
      (return "NewEnumerator4"))
    (:`5`
      (return "NewEnumerator5"))))

(fn `GetStaticMeshAndWallSides`
  (params (X :type Integer) (Y :type Integer))
  (returns (StaticMesh :type "InstancedStaticMeshComponent Object Reference") (Wallsides :type "/Game/GridSystem/StructsAndDataTables/ENUM_WallSides Enum"))
  (bind _output_membervar_0 (break `/Game/GridSystem/StructsAndDataTables/Struct_2DArray` (`|GetArrayItem` (`self.Cells`) X)))
  (bind (_output_material _output_instancedstaticmesh _output_wallsides) (break `/Game/GridSystem/StructsAndDataTables/Struct_CellStruct` (`|GetArrayItem` _output_membervar_0 Y)))
  (`KismetSystemLibrary.PrintString` (`KismetSystemLibrary.GetDisplayName` _output_instancedstaticmesh))
  (return _output_instancedstaticmesh _output_wallsides))

(fn `SpawnArrays`
  (locals (yCoordArray :type "Array of /Game/GridSystem/StructsAndDataTables/Struct_CellStruct Structure") (InstancedStaticMeshToUse :type "InstancedStaticMeshComponent Object Reference"))
  (`KismetArrayLibrary.Array_Clear` (`self.Cells`))
  (for _ (range 1 (+ (`self.Width`) 1))
    (for _index (range 1 (+ (`self.Height`) 1))
      (if (== (mod _index 2) 0)
        (set `local.InstancedStaticMeshToUse` (`self.HexTileInstance`))
        (else
          (set `local.InstancedStaticMeshToUse` (`self.HexTileInstance`))))
      (if (== _index 1)
        (`KismetArrayLibrary.Array_Clear` (`local.yCoordArray`))
        (bind _wallsides (`self.GetRandomWallSides`))
        (set `local.yCoordArray` (`|MakeArray` (make `/Game/GridSystem/StructsAndDataTables/Struct_CellStruct` "/Engine/MapTemplates/Materials/BasicAsset01.BasicAsset01" (`self.HexTileInstance`) _wallsides)))
        (else
          (bind _wallsides_2 (`self.GetRandomWallSides`))
          (`KismetArrayLibrary.Array_Add` (`local.yCoordArray`) (make `/Game/GridSystem/StructsAndDataTables/Struct_CellStruct` "/Engine/MapTemplates/Materials/BasicAsset01.BasicAsset01" (`self.HexTileInstance`) _wallsides_2)))))
    (`KismetArrayLibrary.Array_Add` (`self.Cells`) (make `/Game/GridSystem/StructsAndDataTables/Struct_2DArray` (`local.yCoordArray`)))))

(fn `SpawnGrid`
  (locals (XIndex :type Integer) (YIndex :type Integer) (CellTransform :type "Transform Structure"))
  (bind _tilemesh (`self.TileMesh`))
  (`StaticMeshComponent.SetStaticMesh` (`self.HexTileInstance`) _tilemesh)
  (set `self.Radius_0` (.x (`.Max` (break `Box` (`StaticMesh.GetBoundingBox` _tilemesh)))))
  ;[1 1 1] Width Loop
  (for _index (range 1 (+ (`self.Width`) 1))
    (set `local.XIndex` _index)
    ;[1 1 1] Height Loop
    (for _index_2 (range 1 (+ (`self.Height`) 1))
      (set `local.YIndex` _index_2)
      (bind _returnvalue (`self.CreateCellTransform` (`local.XIndex`) (`local.YIndex`)))
      (set `local.CellTransform` _returnvalue)
      (if (`self.Instanced?`)
        ;[1 1 1] Instanced Mesh
        (bind _returnvalue_2 (`InstancedStaticMeshComponent.AddInstance` (`self.HexTileInstance`) (`local.CellTransform`) false))
        (`KismetArrayLibrary.Array_Add` (`self.TileInstances`) _returnvalue_2)
        (bind (_staticmesh _wallsides) (`self.GetStaticMeshAndWallSides` (`local.XIndex`) (`local.YIndex`)))
        (`self.SpawnWalls` (`local.CellTransform`) _wallsides)
        (else
          ;[1 1 1] Child Actors
          (bind _returnvalue_3 (`AddComponent|NODE_AddChildActorComponent-0` :`RelativeTransform` (`local.CellTransform`)))
          (`ChildActorComponent.SetChildActorClass` _returnvalue_3 "/Game/GridSystem/BluePrints/BP_HexTile.BP_HexTile_C")
          (`self.GetStaticMeshAndWallSides` (`local.XIndex`) (`local.YIndex`))
          (`self.SpawnWalls` (`local.CellTransform`)))))
    ;[1 1 1] Hex-Grid need to offset by the radius every other row so they slot into each other
    (`/Engine/EditorBlueprintResources/StandardMacros.FlipFlop`
      (:`A`
        (set `self.RowOffset` (* (`self.Radius_0`) -1.0)))
      (:`B`
        (set `self.RowOffset` 0.0)))))

(fn `SpawnWalls`
  (params (CellTransform :type "Transform Structure") (WallSides :type "/Game/GridSystem/StructsAndDataTables/ENUM_WallSides Enum" :default "NewEnumerator0"))
  (locals (RowName :type Name))
  (bind _celltransform (`local.CellTransform`))
  (bind _celltransform_2 (`local.CellTransform`))
  (switch `/Game/GridSystem/StructsAndDataTables/ENUM_WallSides` WallSides
    (:`NewEnumerator0`
      (set `local.RowName` "NorthEast"))
    (:`NewEnumerator1`
      (set `local.RowName` "East"))
    (:`NewEnumerator2`
      (set `local.RowName` "SouthEast"))
    (:`NewEnumerator3`
      (set `local.RowName` "SouthWest"))
    (:`NewEnumerator4`
      (set `local.RowName` "West"))
    (:`NewEnumerator5`
      (set `local.RowName` "NorthWest")))
  (bind _returnvalue (`|GetDataTableRow` "/Game/GridSystem/StructsAndDataTables/DT_WallSidesLocation.DT_WallSidesLocation" (`local.RowName`))
    (:`then`
      (if (`self.Instanced?`)
        (bind _returnvalue_2 (`KismetMathLibrary.MakeVector` (+ (.x (.location _celltransform_2)) (break `/Game/GridSystem/StructsAndDataTables/Struct_WallSidesLocation` _returnvalue)) (+ (.y (.location _celltransform_2)) (`.YLocation_10_F8BE951C48D1247C7016F496F8ABBEA2` (break `/Game/GridSystem/StructsAndDataTables/Struct_WallSidesLocation` _returnvalue))) (.z (.location _celltransform_2))))
        (bind _returnvalue_3 (`KismetMathLibrary.MakeRotator` (.roll (.rotation _celltransform)) (.pitch (.rotation _celltransform)) (`.ZRotation_12_6C86AC17459A6B60250730B5668743AB` (break `/Game/GridSystem/StructsAndDataTables/Struct_WallSidesLocation` _returnvalue))))
        (bind _returnvalue_4 (`InstancedStaticMeshComponent.AddInstance` (`self.WallInstance`) (`KismetMathLibrary.MakeTransform` _returnvalue_2 _returnvalue_3) false))
        (`KismetArrayLibrary.Array_Add` (`self.WallInstances`) _returnvalue_4)
        (else
          (bind _returnvalue_5 (`AddComponent|NODE_AddChildActorComponent-1` :`RelativeTransform` (`KismetMathLibrary.MakeTransform` _returnvalue_2 _returnvalue_3)))
          (`ChildActorComponent.SetChildActorClass` _returnvalue_5 "/Game/GridSystem/TileMeshesAndMaterials/BP_Wall.BP_Wall_C"))))))

(fn `UserConstructionScript`
  (`self.SpawnArrays`)
  (`self.SpawnGrid`))