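; Bee actor that travels cell to cell across the hex grid owned by the HexGridManager game mode.
; On BeginPlay it teleports to the first cell, runs AStarPathfinder to a hardcoded end cell, then prints and debug-draws the path.
; Tick, gated by a Delay, plays a Timeline that lerps position and rotation between the last two path nodes, removing the last on finish.
; SetNewActorLocation and an empty FindPath are never called here.
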(event `self.ReceiveBeginPlay`
  (bind _hexcellarray (`HexGridManager.HexCellArray` (`self.As Hex Grid Manager`)))
  (bind _output_ar (break `HexCell2DArraySimulator` (`|GetArrayItem` _hexcellarray)))
  (bind _output_ar_2 (break `HexCell2DArraySimulator` (`|GetArrayItem` (`HexGridManager.HexCellArray` (`self.As Hex Grid Manager`)))))
  (bind _output_ar_3 (break `HexCell2DArraySimulator` (`|GetArrayItem` _hexcellarray 4)))
  (bind _output (`|GetArrayItem` _output_ar_2))
  (bind _ashex_grid_manager (cast `HexGridManager` (`GameplayStatics.GetGameMode`)))
  (set `self.As Hex Grid Manager` _ashex_grid_manager)
  (`KismetSystemLibrary.Delay` 1.0)
  (bind _output_get (set `self.TargetLocation` (`KismetMathLibrary.MakeVector` (.x (.location (`.cellTransform` (break `HexCell` _output)))) (.y (.location (`.cellTransform` (break `HexCell` _output)))) 40.0)))
  (`KismetSystemLibrary.Delay` 1.0)
  (`self.K2_SetActorLocation` _output_get false true)
  (bind _returnvalue (`AStarPathfinder.PathFind` (`self.AStarPathfinder`) _hexcellarray (`|GetArrayItem` _output_ar) (`|GetArrayItem` _output_ar_3 4)))
  (bind _output_get_2 (set `self.PathToFollow` _returnvalue))
  (for (_array_element _array_index) _output_get_2
    (`KismetSystemLibrary.PrintString` (`KismetTextLibrary.Conv_TextToString` (`|FormatText` "Node: {x}, {y}" (break `HexCell` _array_element) (`.Y` (break `HexCell` _array_element)))) true true (struct :`G` 0.66 :`B` 1.0 :`A` 1.0) 40.0)
    (bind _returnvalue_2 (+ _array_index 1))
    (if (not (== _returnvalue_2 (`KismetArrayLibrary.Array_Length` _output_get_2)))
      (`KismetSystemLibrary.DrawDebugLine` (`KismetMathLibrary.MakeVector` (.x (.location (`.cellTransform` (break `HexCell` _array_element)))) (.y (.location (`.cellTransform` (break `HexCell` _array_element)))) (+ (.z (.location (`.cellTransform` (break `HexCell` _array_element)))) 60.0)) (`KismetMathLibrary.MakeVector` (.x (.location (`.cellTransform` (break `HexCell` (`|GetArrayItem` _output_get_2 _returnvalue_2))))) (.y (.location (`.cellTransform` (break `HexCell` (`|GetArrayItem` _output_get_2 _returnvalue_2))))) (+ (.z (.location (`.cellTransform` (break `HexCell` (`|GetArrayItem` _output_get_2 _returnvalue_2))))) 60.0)) (struct) 20.0 4.0))))

(event `self.ReceiveTick`
  (params (DeltaSeconds :type "Float (single-precision)"))
  (bind _pathtofollow (`self.PathToFollow`))
  (bind _returnvalue (`KismetArrayLibrary.Array_Length` (`self.PathToFollow`)))
  (`KismetSystemLibrary.Delay` 2.0)
  (if (== _returnvalue 0)
    _
    (elif (>= _returnvalue 2)
      (bind _direction (`self.GetVector`))
      (bind (_direction_2 _zero_one_lerp _rotatetodirection) (`Timeline|Timeline` :!via `PlayFromStart`)
        (:`Update`
          (`self.K2_SetActorLocation` (`KismetMathLibrary.VLerp` (`self.PointA`) (`self.PointB`) _zero_one_lerp))
          (`self.K2_SetActorRotation` (`KismetMathLibrary.RLerp` (`self.K2_GetActorRotation`) _direction _rotatetodirection)))
        (:`Finished`
          (`KismetArrayLibrary.Array_Remove` _pathtofollow (`KismetArrayLibrary.Array_LastIndex` _pathtofollow)))))))

(fn `FindPath`)

(fn `GetVector`
  (returns (Direction :type "Rotator Structure"))
  (locals (NewLocalVar :type "Rotator Structure" :default (struct)))
  (bind _pathtofollow (`self.PathToFollow`))
  (bind _pathtofollow_2 (`self.PathToFollow`))
  (bind _output (`|GetArrayItem` _pathtofollow_2 (`KismetArrayLibrary.Array_LastIndex` _pathtofollow_2)))
  (bind _output_2 (`|GetArrayItem` _pathtofollow (- (`KismetArrayLibrary.Array_LastIndex` _pathtofollow) 1)))
  (set `self.PointA` (`KismetMathLibrary.MakeVector` (.x (.location (`.cellTransform` (break `HexCell` _output)))) (.y (.location (`.cellTransform` (break `HexCell` _output)))) 50.0))
  (set `self.PointB` (`KismetMathLibrary.MakeVector` (.x (.location (`.cellTransform` (break `HexCell` _output_2)))) (.y (.location (`.cellTransform` (break `HexCell` _output_2)))) 50.0))
  (return (`KismetMathLibrary.Conv_VectorToRotator` (- (`self.PointA`) (`self.PointB`)))))

(fn `SetNewActorLocation`
  (bind _pathtofollow (`self.PathToFollow`))
  (bind _pathtofollow_2 (`self.PathToFollow`))
  (bind _returnvalue_location (`KismetMathLibrary.BreakTransform` (`SceneComponent.K2_GetComponentToWorld` (`self.SkeletalMesh`))))
  (bind _returnvalue_location_2 (`KismetMathLibrary.BreakTransform` (`SceneComponent.K2_GetComponentToWorld` (`self.SkeletalMesh`))))
  (bind _returnvalue_location_3 (`KismetMathLibrary.BreakTransform` (`SceneComponent.K2_GetComponentToWorld` (`self.SkeletalMesh`))))
  (bind (_output_x _output_y _output_celltransform) (break `HexCell` (`|GetArrayItem` _pathtofollow_2 (`KismetArrayLibrary.Array_LastIndex` _pathtofollow_2))))
  (if (== _returnvalue_location_2 (`self.TargetLocation`) :`ErrorTolerance` 0.5)
    (set `self.Direction` (0.0 0.0 0.0))
    (if (not (== (`KismetArrayLibrary.Array_Length` (`self.PathToFollow`)) 0))
      (bind _output_get (set `self.TargetLocation` (`KismetMathLibrary.MakeVector` (.x (.location _output_celltransform)) (.y (.location _output_celltransform)) 40.0)))
      (set `self.Direction` (`KismetMathLibrary.GetDirectionUnitVector` _returnvalue_location _output_get))
      (`KismetArrayLibrary.Array_Remove` _pathtofollow (`KismetArrayLibrary.Array_LastIndex` _pathtofollow)))
    (else
      (set `self.Direction` (`KismetMathLibrary.GetDirectionUnitVector` _returnvalue_location_3 (`self.TargetLocation`))))))

(fn `UserConstructionScript`)