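; Hex grid builder that spawns tiles and walls as mesh instances at BeginPlay from the cell array populated by the HexGridManager game mode.
; SpawnGrid places cells by radius and spacing, staggering alternate rows.
; Each cell's wall-side bitflags select offsets and yaw from DT_WallSidesLocation for its wall instances.
; The grid is written back to the manager as nested struct arrays holding transforms, instance indices and wall flags.
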(event `self.ReceiveBeginPlay`
  (bind _ashex_grid_manager (cast `HexGridManager` (`GameplayStatics.GetGameMode`)))
  (bind _output_get (set `self.As Hex Grid Manager` _ashex_grid_manager))
  (`HexGridManager.PopulateArray` _output_get "/Game/HexGridSystem/TileMeshesAndMaterials/SM_HexTile.SM_HexTile")
  (`self.SpawnGrid`))

(fn `CreateCellTransform`
  (params (XIndex :type Integer) (YIndex :type Integer) (RowOffset :type "Float (double-precision)"))
  (returns (ReturnValue :type "Transform Structure"))
  (bind _yindex (`local.YIndex`))
  (bind _xindex (`local.XIndex`))
  (bind _offset (`self.Offset`))
  (return (`KismetMathLibrary.MakeTransform` (`KismetMathLibrary.MakeVector` (+ (`local.RowOffset`) (* _yindex (`HexGridManager.Radius` (`self.As Hex Grid Manager`)) 2.0) (* _yindex _offset)) (+ (* _offset _xindex) (* _xindex 1.5 (/ (* (`HexGridManager.Radius` (`self.As Hex Grid Manager`)) 2.0) (`KismetMathLibrary.Sqrt` 3.0))))))))

(fn `SpawnGrid`
  (locals (`Row Offset` :type "Float (double-precision)") (XIndex :type Integer) (YIndex :type Integer) (NewOuterArray :type "Array of HexCell2DArraySimulator Structure") (NewInnerArray :type "Array of HexCell Structure") (eWallSidesTemp :type Integer))
  (for (_array_element _array_index) (`HexGridManager.HexCellArray` (`self.As Hex Grid Manager`))
    (set `local.XIndex` _array_index)
    (for (_array_element_2 _array_index_2) (break `HexCell2DArraySimulator` _array_element)
      (set `local.eWallSidesTemp` (`.eWallSidesBits` (break `HexCell` _array_element_2)))
      (set `local.YIndex` _array_index_2)
      (bind _returnvalue (`self.CreateCellTransform` (`local.XIndex`) (`local.YIndex`) (`local.Row Offset`)))
      (`StaticMeshComponent.SetStaticMesh` (`self.HexTileInstance`) (`.StaticMesh` (break `HexCell` _array_element_2)))
      (bind _returnvalue_2 (`InstancedStaticMeshComponent.AddInstance` (`self.HexTileInstance`) _returnvalue false))
      (bind _wallinstances (`self.SpawnWalls` (`local.eWallSidesTemp`) _returnvalue))
      (if (== (`local.YIndex`) 0)
        (bind _hexcell (make `HexCell` (`local.XIndex`) (`local.YIndex`) _returnvalue _returnvalue_2 _wallinstances (`local.eWallSidesTemp`)))
        (set `local.NewInnerArray` (`|MakeArray` _hexcell))
        (else
          (`KismetArrayLibrary.Array_Add` (`local.NewInnerArray`) _hexcell))))
    (if (== (`local.XIndex`) 0)
      (set `local.NewOuterArray` (`|MakeArray` (make `HexCell2DArraySimulator` (`local.NewInnerArray`))))
      (else
        (`KismetArrayLibrary.Array_Add` (`local.NewOuterArray`) (make `HexCell2DArraySimulator` (`local.NewInnerArray`)))))
    (`/Engine/EditorBlueprintResources/StandardMacros.FlipFlop`
      (:`A`
        (set `local.Row Offset` (* (`HexGridManager.Radius` (`self.As Hex Grid Manager`)) -1.0)))
      (:`B`
        (set `local.Row Offset` 0.0))))
  (set `HexGridManager.HexCellArray` (`local.NewOuterArray`) (`self.As Hex Grid Manager`)))

(fn `SpawnWalls`
  (params (WallSides :type Integer) (CellTransform :type "Transform Structure"))
  (returns (WallInstances :type "Array of Integer"))
  (locals (LocalWallInstances :type "Array of Integer"))
  (set `local.LocalWallInstances` (`|MakeArray` 0))
  (bind _returntransforms1 (`self.Wall Transform` (`local.WallSides`) (`local.CellTransform`)))
  (if (not (== (`KismetArrayLibrary.Array_Length` _returntransforms1) 0))
    (for _array_element _returntransforms1
      (bind _returnvalue (`InstancedStaticMeshComponent.AddInstance` (`self.WallInstance`) _array_element false))
      (`KismetArrayLibrary.Array_Add` (`local.LocalWallInstances`) _returnvalue))
    (return (`local.LocalWallInstances`))))

(fn `UserConstructionScript`)

(fn `Wall Transform`
  (params (ValueToCheck :type Integer) (CellTransform :type "Transform Structure"))
  (returns (ReturnTransforms1 :type "Array of Transform Structure"))
  (locals (ReturnTransforms :type "Array of Transform Structure"))
  (bind _celltransform (`local.CellTransform`))
  (bind _celltransform_2 (`local.CellTransform`))
  (set `local.ReturnTransforms` (`|MakeArray` (struct) :!type "Transform Structure"))
  (bind _enumvalue (foreach `EWallSidesBits` false)
    (:`LoopBody`
      (bind _returnvalue (`HexGridManager.HasFlag` (`self.As Hex Grid Manager`) (`KismetMathLibrary.Conv_ByteToInt` _enumvalue) (`local.ValueToCheck`)))
      (if _returnvalue
        (bind _returnvalue_2 (`|GetDataTableRow` "/Game/HexGridSystem/StructsAndDataTables/DT_WallSidesLocation.DT_WallSidesLocation" (`|GetEnumeratorName` _enumvalue))
          (:`then`
            (`KismetArrayLibrary.Array_Add` (`local.ReturnTransforms`) (`KismetMathLibrary.MakeTransform` (`KismetMathLibrary.MakeVector` (+ (.x (.location _celltransform_2)) (break `/Game/HexGridSystem/StructsAndDataTables/Struct_WallSidesLocation` _returnvalue_2)) (+ (.y (.location _celltransform_2)) (`.YLocation_10_F8BE951C48D1247C7016F496F8ABBEA2` (break `/Game/HexGridSystem/StructsAndDataTables/Struct_WallSidesLocation` _returnvalue_2))) (.z (.location _celltransform_2))) (`KismetMathLibrary.MakeRotator` (.roll (.rotation _celltransform)) (.pitch (.rotation _celltransform)) (+ (`.ZRotation_12_6C86AC17459A6B60250730B5668743AB` (break `/Game/HexGridSystem/StructsAndDataTables/Struct_WallSidesLocation` _returnvalue_2)) (.yaw (.rotation _celltransform))))))))))
    (:`then`
      (return (`local.ReturnTransforms`)))))