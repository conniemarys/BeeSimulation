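; Pathfinding Blueprint that, as written, only caches data from the level's hex grid; it contains no path search logic.
; On BeginPlay it finds the BP_HexGrid actor, then RetrieveVariables copies its height, width and cells if the reference is valid.
; It also derives InnerRadius as twice the grid's Radius divided by the square root of three.
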(event `self.ReceiveBeginPlay`
  (bind _returnvalue (`GameplayStatics.GetActorOfClass` "/Game/GridSystem/BluePrints/BP_HexGrid.BP_HexGrid_C"))
  (set `self.HexGrid` _returnvalue)
  (`self.RetrieveVariables`))

(fn `RetrieveVariables`
  (bind _hexgrid (`self.HexGrid`)
    (:`then`
      (set `self.Height` (`/Game/GridSystem/BluePrints/BP_HexGrid.Height` _hexgrid))
      (set `self.Width` (`/Game/GridSystem/BluePrints/BP_HexGrid.Width` _hexgrid))
      (set `self.InnerRadius` (/ (* (`/Game/GridSystem/BluePrints/BP_HexGrid.Radius` _hexgrid) 2.0) (`KismetMathLibrary.Sqrt` 3.0)))
      (set `self.Cells` (`/Game/GridSystem/BluePrints/BP_HexGrid.Cells` _hexgrid)))
    (:`else`)))